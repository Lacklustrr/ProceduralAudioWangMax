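; A trigger volume that switches the Soundscape subsystem's Active state on when an actor begins overlapping it and clears it on exit.
; The live overlap events use the fixed SoundScape.Active tag, with no filter on the overlapping actor.
; BeginPlay derives a palette collection name from the SoundscapeState tag, but only disconnected logic uses it.
; That unused logic would add or remove a palette collection, toggle the configured state and optionally print debug messages.
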(event `self.ReceiveActorBeginOverlap`
  (params (OtherActor :type "Actor Object Reference"))
  (`SoundscapeSubsystem.SetState` (subsystem `SoundscapeSubsystem`) (struct :`TagName` "SoundScape.Active")))

(event `self.ReceiveBeginPlay`
  (set `self.Palette Collection Name` (`BlueprintGameplayTagLibrary.GetTagName` (`self.Soundscape State`))))

(event `self.ReceiveActorEndOverlap`
  (params (OtherActor :type "Actor Object Reference"))
  (`SoundscapeSubsystem.ClearState` (subsystem `SoundscapeSubsystem`) (struct :`TagName` "SoundScape.Active")))

(fn `UserConstructionScript`)