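; Ribadulequin cannon prop that fires cosmetically when anything begins overlapping its Box trigger.
; The overlap plays the one-shot firing animation and sound cue and activates the first muzzle VFX immediately.
; A Sequence starts a separate, equal short Delay for each remaining VFX component, so those effects activate together shortly after the first rather than staggered.
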(event `self.Box.OnComponentBeginOverlap`
  (params (OverlappedComponent :type "PrimitiveComponent Object Reference") (OtherActor :type "Actor Object Reference") (OtherComp :type "PrimitiveComponent Object Reference") (OtherBodyIndex :type Integer) (bFromSweep :type Boolean) (SweepResult :type "HitResult Structure (by ref)"))
  (`SkeletalMeshComponent.PlayAnimation` (`self.Ribadulequin`) "/Game/MedievalCannons/Props/Ribadulequin/AS_Ribadulequin_Anim.AS_Ribadulequin_Anim" false)
  (`AudioComponent.Play` (`self.SFXcue_Firing_Ribadulequin`) 0.0)
  (`ActorComponent.Activate` (`self.VFX_Firing_Ribadulequin_1`) false)
  (`|ExecutionSequence`
    (:`then_0`
      (`KismetSystemLibrary.Delay` 0.2)
      (`ActorComponent.Activate` (`self.VFX_Firing_Ribadulequin_2`) false))
    (:`then_1`
      (`KismetSystemLibrary.Delay` 0.2)
      (`ActorComponent.Activate` (`self.VFX_Firing_Ribadulequin_3`) false))
    (:`then_2`
      (`KismetSystemLibrary.Delay` 0.2)
      (`ActorComponent.Activate` (`self.VFX_Firing_Ribadulequin_4`) false))
    (:`then_3`
      (`KismetSystemLibrary.Delay` 0.2)
      (`ActorComponent.Activate` (`self.VFX_Firing_Ribadulequin_5`) false))
    (:`then_4`
      (`KismetSystemLibrary.Delay` 0.2)
      (`ActorComponent.Activate` (`self.VFX_Firing_Ribadulequin_6`) false))
    (:`then_5`
      (`KismetSystemLibrary.Delay` 0.2)
      (`ActorComponent.Activate` (`self.VFX_Firing_Ribadulequin_7`) false))
    (:`then_6`
      (`KismetSystemLibrary.Delay` 0.2)
      (`ActorComponent.Activate` (`self.VFX_Firing_Ribadulequin_8`) false))
    (:`then_7`
      (`KismetSystemLibrary.Delay` 0.2)
      (`ActorComponent.Activate` (`self.VFX_Firing_Ribadulequin_9`) false))))

(fn `UserConstructionScript`)